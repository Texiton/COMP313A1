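; GetObjective is an interactable actor that shows a note and advances the HUD objective.
; Overlap enables its input, and left mouse flip-flops between adding and removing a NoteHUD widget.
; Opening calls ViewingNote on the HUDController found in the level and sets ViewedLetter; closing calls CollectingTrash.
; Ending overlap disables input and, once viewed, reuses the close path without resetting the FlipFlop.
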(event `Key|LeftMouseButton`
  (params (Key :type "Key Structure"))
  (:`Pressed`
    (`/Engine/EditorBlueprintResources/StandardMacros.FlipFlop`
      (:`A`
        (bind _returnvalue (`|CreateWidget` "/Game/Blueprints/HUD/NoteHUD.NoteHUD_C"))
        (`UserWidget.AddToViewport` _returnvalue 0)
        (bind _outactors (`GameplayStatics.GetAllActorsOfClass` "/Game/Blueprints/HUD/HUDController.HUDController_C"))
        (bind _ashudcontroller (cast `/Game/Blueprints/HUD/HUDController` (`|GetArrayItem` _outactors)))
        (`/Game/Blueprints/HUD/HUDController.ViewingNote` _ashudcontroller)
        (set `self.ViewedLetter` true))
      (:`B`
        (`Widget.RemoveFromParent` _returnvalue :!label _label)
        (bind _outactors_2 (`GameplayStatics.GetAllActorsOfClass` "/Game/Blueprints/HUD/HUDController.HUDController_C"))
        (bind _ashudcontroller_2 (cast `/Game/Blueprints/HUD/HUDController` (`|GetArrayItem` _outactors_2)))
        (if (`self.ViewedLetter`)
          (`/Game/Blueprints/HUD/HUDController.CollectingTrash` _ashudcontroller_2))))))

(event `self.ReceiveActorBeginOverlap`
  (params (OtherActor :type "Actor Object Reference"))
  (`self.EnableInput` (`GameplayStatics.GetPlayerController` 0)))

(event `self.ReceiveActorEndOverlap`
  (params (OtherActor :type "Actor Object Reference"))
  (`self.DisableInput` (`GameplayStatics.GetPlayerController` 0))
  (if (`self.ViewedLetter`)
    (goto _label)))

(fn `UserConstructionScript`)