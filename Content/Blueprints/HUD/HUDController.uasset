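; HUD class that draws the crosshair and manages the intro and trash-collecting UI.
; DrawHUD paints a small white square over a black one at screen center while the PlayerCharacter holds no object.
; LevelBegin shows the InitialHUD widget and ViewingNote removes it.
; CollectingTrash adds a new CollectingTrash widget on each call and plays a song only the first time.
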(event `self.ReceiveDrawHUD`
  (params (SizeX :type Integer) (SizeY :type Integer))
  (bind _returnvalue (`KismetMathLibrary.Conv_IntToDouble` (/ SizeX 2)))
  (bind _returnvalue_2 (`KismetMathLibrary.Conv_IntToDouble` (/ SizeY 2)))
  ;[1 1 1] Draw Crosshair
  (bind _asplayer_character (cast `/Game/Blueprints/PlayerCharacter` (`GameplayStatics.GetPlayerPawn` 0)))
  (if (not (`/Game/Blueprints/PlayerCharacter.IsHoldingObject` _asplayer_character))
    (`self.DrawRect` self (struct :`A` 1.0) _returnvalue _returnvalue_2 4.0 4.0)
    (`self.DrawRect` (struct :`R` 1.0 :`G` 1.0 :`B` 1.0 :`A` 1.0) _returnvalue _returnvalue_2 3.0 3.0)))

(event `CollectingTrash`
  ;[1 1 1] Draw Collecting Trash UI
  (bind _returnvalue (`|CreateWidget` "/Game/Blueprints/HUD/CollectingTrash.CollectingTrash_C"))
  (`UserWidget.AddToViewport` _returnvalue 0)
  (`/Engine/EditorBlueprintResources/StandardMacros.DoOnce` false
    (:`Completed`
      (`GameplayStatics.PlaySound2D` "/Game/Audio/song.song" 1.0 1.0 0.0 null null))))

(event `ViewingNote`
  ;[1 1 1] Draw Initial UI
  (`Widget.RemoveFromParent` (stale `LevelBegin` _returnvalue)))

(event `LevelBegin`
  ;[1 1 1] Draw Initial UI
  (bind _returnvalue (`|CreateWidget` "/Game/Blueprints/HUD/InitialHUD.InitialHUD_C"))
  (`UserWidget.AddToViewport` _returnvalue 0))

(fn `UserConstructionScript`)