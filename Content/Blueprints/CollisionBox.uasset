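; CollisionBox is a scoring trigger that counts objects entering its Cylinder and checks for a win, apparently for trash disposal.
; Any overlapping actor adds a point to the player character's Score, is destroyed without a type check, and triggers a trash impact sound.
; Once Score reaches the hard-coded threshold, it shows the WinningScreen widget and switches input to UI only.
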(event `self.Cylinder.OnComponentBeginOverlap`
  (params (OverlappedComponent :type "PrimitiveComponent Object Reference") (OtherActor :type "Actor Object Reference") (OtherComp :type "PrimitiveComponent Object Reference") (OtherBodyIndex :type Integer) (bFromSweep :type Boolean) (SweepResult :type "HitResult Structure (by ref)"))
  (bind _returnvalue (`GameplayStatics.GetPlayerPawn` 0))
  (bind _asplayer_character (cast `/Game/Blueprints/PlayerCharacter` _returnvalue))
  (set `/Game/Blueprints/PlayerCharacter.Score` (+ (`/Game/Blueprints/PlayerCharacter.Score` _asplayer_character) 1) _asplayer_character)
  (`self.K2_DestroyActor` OtherActor)
  (`GameplayStatics.PlaySoundAtLocation` "/Game/Audio/TrashImpactSFX.TrashImpactSFX" (`SceneComponent.K2_GetComponentLocation` (`self.Cylinder`)) (struct) 1.0 1.0 0.0 null null null)
  ;[1 1 1] Check if player has won
  (bind _asplayer_character_2 (cast `/Game/Blueprints/PlayerCharacter` _returnvalue))
  (if (>= (`/Game/Blueprints/PlayerCharacter.Score` _asplayer_character_2) 15)
    (bind _returnvalue_2 (`|CreateWidget` "/Game/Blueprints/WinningScreen.WinningScreen_C"))
    (`UserWidget.AddToViewport` _returnvalue_2 0)
    (`WidgetBlueprintLibrary.SetInputMode_UIOnlyEx` (`GameplayStatics.GetPlayerController` 0) null)))

(fn `UserConstructionScript`)